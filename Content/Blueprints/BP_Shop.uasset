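; Shop actor that shows the saved shop name, the player's licence displays, purchasable props and animated gates.
; After a short BeginPlay delay it loads the name, caches the player and refreshes licences and props.
; Licence levels reveal meshes cumulatively; purchases set flags that toggle prop visibility and collision for flowers, ATM, helicopter and tank.
; Separate events toggle four document meshes and raise or lower two gates via a timeline.
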(event Custom|OpenDoors
  (bind _newtrack_0 (Timeline|T_Doors Play)
    (:Update
      (Transformation|SetRelativeLocation (Variables|Default|GetGate7) (Math|Vector|MakeVector 1.5e+03 -896.87371 (Math|Float|Lerp 0.0 3e+02 _newtrack_0)) false false)
      (Transformation|SetRelativeLocation (Variables|Default|GetGate) (Math|Vector|MakeVector 1.5e+03 -361.209869 (Math|Float|Lerp 0.0 3e+02 _newtrack_0)) false false))))

(event Custom|CloseDoors
  (bind _newtrack_0 (Timeline|T_Doors Reverse)
    (:Update
      (Transformation|SetRelativeLocation (Variables|Default|GetGate7) (Math|Vector|MakeVector 1.5e+03 -896.87371 (Math|Float|Lerp 0.0 3e+02 _newtrack_0)) false false)
      (Transformation|SetRelativeLocation (Variables|Default|GetGate) (Math|Vector|MakeVector 1.5e+03 -361.209869 (Math|Float|Lerp 0.0 3e+02 _newtrack_0)) false false))))

(event Custom|Updatelicences
  (bind _playerref (Variables|Default|GetPlayerRef)
    (:then
      (switch int (Variables|/Game/Blueprints/Characters/Player/BP_Player.BP_Player_C|GetLicenceLevel _playerref)
        (:1
          _)
        (:2
          (Rendering|SetVisibility (Variables|Default|GetLicenceC) true false :!label _label))
        (:3
          (Rendering|SetVisibility (Variables|Default|GetLicenceB) true false :!label _label_2)
          (goto _label))
        (:4
          (Rendering|SetVisibility (Variables|Default|GetLicenceA) true false)
          (goto _label_2)))
      (Rendering|SetVisibility (Variables|Default|GetLicenceD) true false))
    (:else)))

(event Custom|SetDocumentVisibility
  (params (NewHidden :type Boolean) (Target :type Scene%20Component%20Object%20Reference))
  (Development|SetHiddeninGame Target (not NewHidden) false))

(event Custom|SetAllDocumentsVisibility
  (params (id :type Boolean) (hunting :type Boolean) (licence :type Boolean) (derogation :type Boolean))
  (CallFunction|SetDocumentVisibility id (Variables|Default|GetIdCardMesh1))
  (CallFunction|SetDocumentVisibility hunting (Variables|Default|GetHuntingLicenceMesh))
  (CallFunction|SetDocumentVisibility licence (Variables|Default|GetSportLicenceMesh))
  (CallFunction|SetDocumentVisibility derogation (Variables|Default|GetDerogationMesh)))

(event Custom|SetElements
  (CallFunction|SetElement (Variables|Default|GetHasFlowers?) (Variables|Default|GetFlowerMesh1))
  (CallFunction|SetElement (Variables|Default|GetHasFlowers?) (Variables|Default|GetFlowerMesh))
  (CallFunction|SetElement (Variables|Default|GetHasAtm?) (Variables|Default|GetATMMesh))
  (CallFunction|SetElement (Variables|Default|GetHasHeli?) (Variables|Default|GetHelicopterMesh))
  (CallFunction|SetElement (Variables|Default|GetHasTank?) (Variables|Default|GetTankMesh)))

(event Custom|SetElement
  (params (NewParam :type Boolean) (NewParam2 :type Static%20Mesh%20Component%20Object%20Reference))
  (if NewParam
    (Rendering|SetVisibility NewParam2 true true)
    (Collision|SetCollisionEnabled NewParam2 "QueryAndPhysics")
    (else
      (Rendering|SetVisibility NewParam2 false true)
      (Collision|SetCollisionEnabled NewParam2 "NoCollision"))))

(event Custom|ElementBought
  (params (NewParam :type String))
  (switch string NewParam
    (:Flowers
      (Variables|Default|SetHasFlowers? true))
    (:Atm
      (Variables|Default|SetHasAtm? true))
    (:Helicopter
      (Variables|Default|SetHasHeli? true))
    (:Tank
      (Variables|Default|SetHasTank? true)))
  (CallFunction|SetElements))

(event EventBeginPlay
  (Utilities|FlowControl|Delay 0.2)
  (Utilities|FlowControl|Sequence
    (:then_0
      (bind _returnvalue (SaveGame|DoesSaveGameExist "GameSave"))
      (if _returnvalue
        (bind _returnvalue_2 (SaveGame|LoadGamefromSlot "GameSave"))
        (bind _asbp_game_save (Utilities|Casting|CastToBP_GameSave _returnvalue_2))
        (Rendering|Components|TextRender|SetText (Variables|Default|GetTextRender) (Variables|/Game/Blueprints/Saves/BP_GameSave.BP_GameSave_C|GetShopName _asbp_game_save))))
    (:then_1
      (bind _asbp_player (Utilities|Casting|CastToBP_Player (Game|Player|GetPlayerPawn 0)))
      (Variables|Default|SetPlayerRef _asbp_player))
    (:then_2
      (CallFunction|Updatelicences))
    (:then_3
      (CallFunction|SetElements))))

(fn ConstructionScript)