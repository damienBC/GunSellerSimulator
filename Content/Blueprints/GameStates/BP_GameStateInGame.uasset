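; In-game GameState that runs the shop's day cycle: opening, clock and closing time.
; StartDay opens the shop and its doors, sets the day status and plays a bell followed by game music.
; A looping timer advances the clock during the day and updates the player's HUD.
; At the closing threshold, a DoOnce flips the status, shows the closed sign, resets doors and closes the shop.
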(event Custom|UpdateTime
  (if (Utilities|Enum|Equal(Enum) (Variables|Default|GetDayStatus) "NewEnumerator1")
    (Variables|Default|SetTime (+ (Variables|Default|GetTime) 1))
    (bind _hudref (Variables|/Game/Blueprints/Characters/Player/BP_Player.BP_Player_C|GetHUDRef (Variables|Default|GetPlayerRef))
      (:then
        (Default|UpdateTime _hudref (Variables|Default|GetTime))
        (if (>= (Variables|Default|GetTime) 1140)
          (Utilities|FlowControl|DoOnce false
            (:Completed
              (Variables|Default|SetDayStatus "NewEnumerator2")
              (bind _returnvalue (Actor|GetActorOfClass "/Game/Blueprints/Elements/BP_OpenSign.BP_OpenSign_C"))
              (Default|ShowCloseSign _returnvalue)
              (for _array_element (Variables|Default|GetDoors)
                (Default|ResetDoor _array_element)
                (bind _returnvalue_2 (Actor|GetActorOfClass "/Game/Blueprints/BP_Shop.BP_Shop_C"))
                (Default|CloseDoors _returnvalue_2))))))
      (:else))))

(event Custom|StartDay
  (bind _returnvalue (Actor|GetActorOfClass "/Game/Blueprints/BP_Shop.BP_Shop_C"))
  (Default|OpenDoors _returnvalue)
  (Variables|Default|SetDayStatus "NewEnumerator1")
  (for _array_element (Variables|Default|GetDoors)
    (Default|OpenDoorDuringDay _array_element))
  (Audio|PlaySound2D "/Game/Sounds/SW_bell.SW_bell" 1.0 1.0 0.0 0 0)
  (Utilities|FlowControl|Delay 0.5)
  (Audio|PlaySound2D "/Game/Sounds/Music/SC_GameMusic.SC_GameMusic" 1.0 1.0 0.0 0 0))

(event EventBeginPlay
  (Utilities|FlowControl|Sequence
    (:then_0
      (bind _asbp_player (Utilities|Casting|CastToBP_Player (Game|Player|GetPlayerPawn 0)))
      (Variables|Default|SetPlayerRef _asbp_player))
    (:then_1
      (bind _outactors (Actor|GetAllActorsOfClass "/Game/Blueprints/BP_Door.BP_Door_C"))
      (Variables|Default|SetDoors _outactors))
    (:then_2
      (Utilities|Time|SetTimerbyEvent (delegate Custom|UpdateTime) 0.5 true))))

(fn ConstructionScript)