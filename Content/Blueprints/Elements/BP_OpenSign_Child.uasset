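; Tutorial variant of the open sign that launches the tutorial NPC when interacted with.
; Interact calls the parent behavior, then a DoOnce spawns BP_NPC_Tuto at the Spawner, passing it the shop entry, inside, desk and spawner references, and destroys the TextRender component.
; After a short delay following the spawn, it clears IsTutorial on BP_GameStateInGame.
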(event Custom|SpawnAiTuto
  (bind _spawner (Variables|Default|GetSpawner))
  (Game|SpawnActorfromClass "/Game/Blueprints/Characters/NPC/BP_NPC_Tuto.BP_NPC_Tuto_C" (Math|Transform|MakeTransform (Transformation|GetActorLocation _spawner) "0, 0, 0" "1.000000,1.000000,1.000000") "Undefined" "MultiplyWithRoot" 0 (Variables|Default|GetShop%20Entry) (Variables|Default|GetShop%20Inside) (Variables|Default|GetShop%20Desk) _spawner 0)
  (Utilities|FlowControl|Delay 1e+01)
  (bind _asbp_game_state_in_game (Utilities|Casting|CastToBP_GameStateInGame (Game|GetGameState)))
  (Variables|/Game/Blueprints/GameStates/BP_GameStateInGame.BP_GameStateInGame_C|SetIsTutorial? _asbp_game_state_in_game false))

(event EventBeginPlay
  (|CallParentFunction) ; This node is disabled and will not be called.\nDrag off pins to build functionality.
)

(event Collision|EventActorBeginOverlap
  (params (OtherActor :type Actor%20Object%20Reference)))

(event EventTick
  (params (DeltaSeconds :type Float%20%28single-precision%29)))

(event EventInteract
  (|CallParentFunction)
  (Utilities|FlowControl|DoOnce false
    (:Completed
      (CallFunction|SpawnAiTuto)
      (Components|DestroyComponent (Variables|Default|GetTextRender)))))

(fn ConstructionScript
  (|CallParentFunction))