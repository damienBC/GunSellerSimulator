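; Interactive shelf element with a cardboard container box that opens and closes on interaction and reveals where items of its category can be placed.
; Interact alternates through a FlipFlop between the box's open and close animations, and opening also calls ShowAvailablePlacements.
; That event scans every BP_Placement actor in the level and reveals inactive ones matching the shelf's Category.
; Closing only plays the animation and does not hide revealed placements.
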(event Custom|ShowAvailablePlacements
  (bind _outactors (Actor|GetAllActorsOfClass "/Game/Blueprints/Elements/Placements/BP_Placement.BP_Placement_C"))
  (for _array_element _outactors
    (if (and (== (Variables|/Game/Blueprints/Elements/Placements/BP_Placement.BP_Placement_C|GetIsActivated? _array_element) false) (Utilities|Enum|Equal(Enum) (Variables|/Game/Blueprints/Elements/Placements/BP_Placement.BP_Placement_C|GetCategory _array_element) (Variables|Default|GetCategory)))
      (Default|Reveal _array_element))))

(event EventBeginPlay
  (|CallParentFunction) ; This node is disabled and will not be called.\nDrag off pins to build functionality.
)

(event Collision|EventActorBeginOverlap
  (params (OtherActor :type Actor%20Object%20Reference))
  (|CallParentFunction OtherActor) ; This node is disabled and will not be called.\nDrag off pins to build functionality.
)

(event EventTick
  (params (DeltaSeconds :type Float%20%28single-precision%29))
  (|CallParentFunction DeltaSeconds) ; This node is disabled and will not be called.\nDrag off pins to build functionality.
)

(event EventInteract
  (bind _containerbox (Variables|Default|GetContainerBox))
  (Utilities|FlowControl|FlipFlop
    (:A
      (Components|Animation|PlayAnimation _containerbox "/Game/Fab/CardBoard/source/AB_OpenCardBoard.AB_OpenCardBoard" false)
      (CallFunction|ShowAvailablePlacements))
    (:B
      (Components|Animation|PlayAnimation _containerbox "/Game/Fab/CardBoard/source/AB_CloseCardBoard.AB_CloseCardBoard" false))))

(fn ConstructionScript
  (|CallParentFunction))