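; BP_Interactive_Object_Weapon is an interactive weapon object, represented in its logic by a container box that opens and closes.
; Each Interact event passes through a FlipFlop that alternately plays the open and close animations once on the ContainerBox.
; The graph contains no weapon pickup or equip logic, and the construction script only calls its parent.
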(event EventBeginPlay
  (|CallParentFunction) ; This node is disabled and will not be called.\nDrag off pins to build functionality.
)

(event Collision|EventActorBeginOverlap
  (params (OtherActor :type Actor%20Object%20Reference))
  (|CallParentFunction OtherActor) ; This node is disabled and will not be called.\nDrag off pins to build functionality.
)

(event EventTick
  (params (DeltaSeconds :type Float%20%28single-precision%29))
  (|CallParentFunction DeltaSeconds) ; This node is disabled and will not be called.\nDrag off pins to build functionality.
)

(event EventInteract
  (bind _containerbox (Variables|Default|GetContainerBox))
  (Utilities|FlowControl|FlipFlop
    (:A
      (Components|Animation|PlayAnimation _containerbox "/Game/Fab/WeaponCase/Anim/AM_Open.AM_Open" false))
    (:B
      (Components|Animation|PlayAnimation _containerbox "/Game/Fab/WeaponCase/Anim/AM_Close.AM_Close" false))))

(fn ConstructionScript
  (|CallParentFunction))