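; BP_Placement is an interactable placement spot that starts inactive and, once built, takes in items the player is holding.
; While inactive, Interact accepts only a held DIY-type object, swapping the mesh material and activating the spot.
; Once active, Interact adds the held BP_Interactive_Object to StockedItems and prints the returned index; socket attachment is noted but not implemented.
; Both successful paths call CallDeleteItem on the player.
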(event Custom|PlaceShelf
  (switch Utilities|FlowControl|Switch|SwitchonE_InteractiveTypes (Variables|/Game/Blueprints/Elements/Interactive/BP_Interactive.BP_Interactive_C|GetType (Variables|/Game/Blueprints/Characters/BP_Player.BP_Player_C|GetGrabbedObject (Variables|Default|GetPlayerRef)))
    (:NewEnumerator2
      (Rendering|Material|SetMaterial (Variables|Default|GetStaticMesh) 0 (Variables|Default|GetNewMaterial))
      (Variables|Default|SetIsActivated? true)
      (Default|CallDeleteItem (Variables|Default|GetPlayerRef)))))

(event Custom|PlaceItem
  ;[1 0 0] Will add the item physically via a socket and in the stock
  (bind _asbp_interactive_object (Utilities|Casting|CastToBP_Interactive_Object (Variables|/Game/Blueprints/Characters/BP_Player.BP_Player_C|GetGrabbedObject (Variables|Default|GetPlayerRef))))
  (bind _returnvalue (Utilities|Array|Add (Variables|Default|GetStockedItems) _asbp_interactive_object))
  (Development|PrintString (Utilities|String|ToString(Integer) _returnvalue))
  (Default|CallDeleteItem (Variables|Default|GetPlayerRef)))

(event Collision|EventActorBeginOverlap
  (params (OtherActor :type Actor%20Object%20Reference))
  (|CallParentFunction OtherActor) ; This node is disabled and will not be called.\nDrag off pins to build functionality.
)

(event EventTick
  (params (DeltaSeconds :type Float%20%28single-precision%29))
  (|CallParentFunction DeltaSeconds) ; This node is disabled and will not be called.\nDrag off pins to build functionality.
)

(event EventInteract
  (if (Variables|Default|GetIsActivated?)
    (CallFunction|PlaceItem)
    (else
      (CallFunction|PlaceShelf))))

(fn ConstructionScript
  (|CallParentFunction))