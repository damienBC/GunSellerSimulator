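; BP_OpenSign is an interactable open/closed sign that starts the in-game day.
; On Interact it rotates its static mesh to the open side, calls StartDay on BP_GameStateInGame and then disables the mesh's collision.
; A separate ShowCloseSign event rotates the mesh back to the closed side but leaves collision unchanged.
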(event Custom|ShowOpenSign
  (Transformation|SetRelativeRotation (Variables|Default|GetStaticMesh) "0.000000,180.000000,0.000000" false false))

(event Custom|ShowCloseSign
  (Transformation|SetRelativeRotation (Variables|Default|GetStaticMesh) "0, 0, 0" false false))

(event EventBeginPlay
  (|CallParentFunction))

(event EventInteract
  (CallFunction|ShowOpenSign)
  (bind _asbp_game_state_in_game (Utilities|Casting|CastToBP_GameStateInGame (Game|GetGameState)))
  (Default|StartDay _asbp_game_state_in_game)
  (Collision|SetCollisionEnabled (Variables|Default|GetStaticMesh) "NoCollision"))

(fn ConstructionScript
  (|CallParentFunction))