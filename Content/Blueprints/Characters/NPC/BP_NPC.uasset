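; Shop customer NPC with a random mesh that patrols shuffled active waypoints, seeking a random desired item, then leaves and despawns.
; InspectItem checks a matching item's price against BP_Computer's recommended price and shows interest.
; At the desk it generates random permit documents and offers accept/refuse widgets based on the player's held item.
; Sales update money and popularity, costing a life if documents fail the category check; timeouts lower popularity.
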(event Custom|Patrol
  (bind _currentwaypoint (Variables|Default|GetCurrentWaypoint))
  (bind _activepath (Variables|Default|GetActivePath))
  (bind _output (Utilities|Array|Get(acopy) _activepath _currentwaypoint))
  (Utilities|IsValid _output
    (:Is%20Valid
      (AI|AIMoveTo self "0, 0, 0" _output 5.0 false
        (:OnSuccess
          (Utilities|FlowControl|Delay (Math|Random|RandomFloatinRange 1.0 4.0))
          (Math|Integer|IncrementInt (Variables|Default|GetCurrentWaypoint)
            (:%20%20
              (CallFunction|Patrol))))))
    (:Is%20Not%20Valid
      (CallFunction|QuitShop))))

(event Custom|QuitShop
  (Rendering|SetVisibility (Variables|Default|GetWidget) false false)
  (Variables|Default|SetCycle "NewEnumerator4")
  (AI|AIMoveTo self "0, 0, 0" (Variables|Default|GetShopInside) 5.0 false
    (:OnSuccess
      (AI|AIMoveTo self "0, 0, 0" (Variables|Default|GetShopEntry) 5.0 false
        (:OnSuccess
          (AI|AIMoveTo self "0, 0, 0" (Variables|Default|GetSpawner) 5.0 false
            (:OnSuccess
              (Actor|DestroyActor))))))))

(event Custom|SpawnSuitcase
  (bind _mesh (Variables|Character|GetMesh))
  (bind _returnvalue (Game|SpawnActorfromClass "/Game/Blueprints/Characters/NPC/Assets/BP_suitcase.BP_suitcase_C" (Transformation|GetSocketTransform _mesh "Bag" "RTS_World") "Undefined" "MultiplyWithRoot" 0 0))
  (Transformation|AttachComponentToComponent _returnvalue _mesh "Bag" "SnapToTarget" "SnapToTarget" "SnapToTarget" true))

(event Custom|GenerateDocuments
  (Variables|Default|SetHasId? (Math|Random|RandomBool))
  (Variables|Default|SetHasHunting? (Math|Random|RandomBool))
  (Variables|Default|SetHasWeaponLicence? (Math|Random|RandomBool))
  (Variables|Default|SetHasDerogation? (Math|Random|RandomBool)))

(event Custom|Test
  (Variables|Default|SetCycle "NewEnumerator2")
  (Rendering|SetVisibility (Variables|Default|GetWidget) false false)
  (AI|AIMoveTo self "0, 0, 0" (Variables|Default|GetShopDesk) 5.0 false
    (:OnSuccess
      (CallFunction|ChangeWidget)
      (Variables|Default|SetCycle "NewEnumerator3")
      (CallFunction|GenerateDocuments)
      (bind _returnvalue (Actor|GetActorOfClass "/Game/Blueprints/BP_Shop.BP_Shop_C"))
      (Default|SetAllDocumentsVisibility _returnvalue (Variables|Default|GetHasId?) (Variables|Default|GetHasHunting?) (Variables|Default|GetHasWeaponLicence?) (Variables|Default|GetHasDerogation?))
      (Utilities|FlowControl|Delay 15.0)
      (if (Utilities|Enum|NotEqual(Enum) (Variables|Default|GetCycle) "NewEnumerator4")
        (bind _asbp_player (Utilities|Casting|CastToBP_Player (Game|GetPlayerCharacter 0))
          (:then
            (Default|ChanePopularity _asbp_player -5))
          (:CastFailed
            _))
        (CallFunction|QuitShop)))))

(event Custom|ChangeWidget
  (bind _self self)
  (bind _widget (Variables|Default|GetWidget))
  (bind _asbp_player (Utilities|Casting|CastToBP_Player (Game|GetPlayerCharacter 0)))
  (bind _grabbedobject (Variables|/Game/Blueprints/Characters/Player/BP_Player.BP_Player_C|GetGrabbedObject _asbp_player)
    (:then
      (if (== (Variables|Default|GetItemLookingFor) (Utilities|GetClass _grabbedobject))
        (bind _asbp_interactive_solo (Utilities|Casting|CastToBP_Interactive_Solo (Variables|Default|GetStocked%20Items)))
        (Widget|RemovefromParent (UserInterface|GetUserWidgetObject _widget))
        (bind _returnvalue (UserInterface|CreateWidget "/Game/Blueprints/Widgets/InGameWidgets/NPCWidgets/WBP_AcceptSell.WBP_AcceptSell_C" 0 _self (Variables|/Game/Blueprints/Elements/Interactive/SoloItems/BP_Interactive_Solo.BP_Interactive_Solo_C|GetImageLogo _asbp_interactive_solo)))
        (UserInterface|SetWidget _widget _returnvalue)
        (else
          (bind _asbp_interactive_solo_2 (Utilities|Casting|CastToBP_Interactive_Solo (Variables|Default|GetStocked%20Items) :!label _label))
          (Utilities|IsValid _asbp_interactive_solo_2
            (:Is%20Valid
              (bind _returnvalue_2 (UserInterface|CreateWidget "/Game/Blueprints/Widgets/InGameWidgets/NPCWidgets/WBP_RefuseSell.WBP_RefuseSell_C" 0 _self (Variables|/Game/Blueprints/Elements/Interactive/SoloItems/BP_Interactive_Solo.BP_Interactive_Solo_C|GetImageLogo _asbp_interactive_solo_2)))
              (UserInterface|SetWidget _widget _returnvalue_2))
            (:Is%20Not%20Valid
              _)))))
    (:else
      (goto _label)))
  (Rendering|SetVisibility (Variables|Default|GetWidget) true false))

(event Custom|RefuseBuy
  (CallFunction|QuitShop)
  (CallFunction|ChangeWidget)
  (bind _returnvalue (Actor|GetActorOfClass "/Game/Blueprints/BP_Shop.BP_Shop_C"))
  (Default|SetAllDocumentsVisibility _returnvalue false false false false))

(event Custom|MakeTransaction
  (bind _asbp_player (Utilities|Casting|CastToBP_Player (Game|GetPlayerCharacter 0)))
  (bind _asbp_interactive_solo (Utilities|Casting|CastToBP_Interactive_Solo (Variables|/Game/Blueprints/Characters/Player/BP_Player.BP_Player_C|GetGrabbedObject _asbp_player)))
  (bind _newparam (CallFunction|ChecktransactionFunc _asbp_interactive_solo))
  (if _newparam
    _
    (else
      (Default|LoseLife _asbp_player)))
  (Default|UpdateMoney _asbp_player (Variables|/Game/Blueprints/Elements/Interactive/SoloItems/BP_Interactive_Solo.BP_Interactive_Solo_C|GetPrice _asbp_interactive_solo))
  (bind _returnvalue (Actor|GetActorOfClass "/Game/Blueprints/BP_Shop.BP_Shop_C"))
  (Default|UpdateSells _returnvalue (Variables|/Game/Blueprints/Elements/Interactive/SoloItems/BP_Interactive_Solo.BP_Interactive_Solo_C|GetPrice _asbp_interactive_solo))
  (Default|ChanePopularity _asbp_player 5)
  (Default|CallDeleteItem _asbp_player)
  (CallFunction|SpawnSuitcase)
  (CallFunction|QuitShop)
  (CallFunction|ChangeWidget)
  (bind _returnvalue_2 (Actor|GetActorOfClass "/Game/Blueprints/BP_Shop.BP_Shop_C"))
  (Default|SetAllDocumentsVisibility _returnvalue_2 false false false false))

(event EventBeginPlay
  (Utilities|FlowControl|Sequence
    (:then_0
      (bind _aswbp_interested (Utilities|Casting|CastToWBP_Interested (UserInterface|GetUserWidgetObject (Variables|Default|GetWidget))))
      (Variables|/Game/Blueprints/Widgets/InGameWidgets/NPCWidgets/WBP_Interested.WBP_Interested_C|SetNPCRef _aswbp_interested self)
      (Rendering|SetVisibility (Variables|Default|GetWidget) false false)
      (AI|AIMoveTo self "0, 0, 0" (Variables|Default|GetShopEntry) 5.0 false
        (:OnSuccess
          (AI|AIMoveTo self (Transformation|GetActorLocation (Variables|Default|GetShopInside)) 0 5.0 false
            (:OnSuccess
              (bind _outactors (Actor|GetAllActorsOfClass "/Game/Blueprints/Characters/NPC/BP_WayPoint.BP_WayPoint_C"))
              (for _array_element _outactors
                (if (Variables|/Game/Blueprints/Characters/NPC/BP_WayPoint.BP_WayPoint_C|GetIsActive? _array_element)
                  (Utilities|Array|Add (Variables|Default|GetActivePath) _array_element)))
              (Utilities|Array|Shuffle (Variables|Default|GetActivePath))
              (CallFunction|Patrol))
            (:OnFail
              (Development|PrintString "Hello"))))))
    (:then_1
      (Variables|Default|SetItemLookingFor (.OutItem (Utilities|Array|Random (Variables|Default|GetListOfDesirableItems)))))))

(event Custom|InspectItem
  (params (NewParam :type BP%20Placement%20Object%20Reference))
  (bind _stockeditems (Variables|/Game/Blueprints/Elements/Placements/BP_Placement.BP_Placement_C|GetStockedItems NewParam)
    (:then
      (Variables|Default|SetStocked%20Items _stockeditems)
      (if (== (Variables|Default|GetItemLookingFor) (Utilities|GetClass _stockeditems))
        (AI|AIMoveTo self "0, 0, 0" NewParam 5e+01 false
          (:OnSuccess
            (Variables|Default|SetCycle "NewEnumerator1")
            (bind _aswbp_interested (Utilities|Casting|CastToWBP_Interested (UserInterface|GetUserWidgetObject (Variables|Default|GetWidget))))
            (bind _asbp_interactive_solo (Utilities|Casting|CastToBP_Interactive_Solo (Variables|Default|GetStocked%20Items)))
            (bind _newparam (CallFunction|AcceptItemPrice _asbp_interactive_solo))
            (if _newparam
              (Variables|/Game/Blueprints/Widgets/InGameWidgets/NPCWidgets/WBP_Interested.WBP_Interested_C|SetIn%20Brush%20Image _aswbp_interested (Variables|/Game/Blueprints/Elements/Interactive/SoloItems/BP_Interactive_Solo.BP_Interactive_Solo_C|GetImageLogo _asbp_interactive_solo))
              (Default|UpdateBrush _aswbp_interested)
              (Rendering|SetVisibility (Variables|Default|GetWidget) true false)
              (Utilities|FlowControl|Delay 15.0)
              (if (Utilities|Enum|Equal(Enum) (Variables|Default|GetCycle) "NewEnumerator1")
                (bind _asbp_player (Utilities|Casting|CastToBP_Player (Game|GetPlayerCharacter 0))
                  (:then
                    (Default|ChanePopularity _asbp_player -5))
                  (:CastFailed
                    _))
                (CallFunction|QuitShop :!label _label))
              (else
                (Development|PrintString "Hello")
                (goto _label)))))))
    (:else)))

(fn ConstructionScript
  (Components|SkeletalMesh|SetSkeletalMeshAsset (Variables|Character|GetMesh) (.OutItem (Utilities|Array|Random (Variables|Default|GetMeshes))))
  (Variables|/Script/Engine.CharacterMovementComponent|SetMaxWalkSpeed (Variables|Character|GetCharacterMovement) 2.5e+02))

(fn ChecktransactionFunc
  (params (Target :type BP%20Interactive%20Object%20Reference))
  (switch Utilities|FlowControl|Switch|SwitchonE_Categories (Variables|/Game/Blueprints/Elements/Interactive/BP_Interactive.BP_Interactive_C|GetCategory Target)
    (:NewEnumerator0
      (return (Utilities|AValid?)))
    (:NewEnumerator1
      (return (Utilities|BValid?)))
    (:NewEnumerator2
      (return (Utilities|CValid?)))
    (:NewEnumerator3
      (return (Utilities|DorItemValid?)))))

(fn AcceptItemPrice
  (params (Object :type BP%20Interactive%20Solo%20Object%20Reference))
  (bind _price (Variables|/Game/Blueprints/Elements/Interactive/SoloItems/BP_Interactive_Solo.BP_Interactive_Solo_C|GetPrice Object))
  (bind _returnvalue (Actor|GetActorOfClass "/Game/Blueprints/BP_Computer.BP_Computer_C"))
  (if (.ReturnValue (Utilities|Map|Find (Variables|/Game/Blueprints/BP_Computer.BP_Computer_C|GetRecommandedPriceList _returnvalue) (Utilities|GetClass Object)))
    (if (<= _price (.Value (Utilities|Map|Find (Variables|/Game/Blueprints/BP_Computer.BP_Computer_C|GetRecommandedPriceList _returnvalue) (Utilities|GetClass Object))))
      (return true)
      (else
        (return (>= (/ (- _price (.Value (Utilities|Map|Find (Variables|/Game/Blueprints/BP_Computer.BP_Computer_C|GetRecommandedPriceList _returnvalue) (Utilities|GetClass Object)))) (.Value (Utilities|Map|Find (Variables|/Game/Blueprints/BP_Computer.BP_Computer_C|GetRecommandedPriceList _returnvalue) (Utilities|GetClass Object)))) (Math|Random|RandomFloatinRange 0.0 1e+02)))))))